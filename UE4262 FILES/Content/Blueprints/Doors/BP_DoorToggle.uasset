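; BP_DoorToggle is a door that opens and closes along its Z axis according to the state of a linked lever.
; On BeginPlay it finds the BP_Lever whose LeverIdentifier matches its DoorIdentifier and caches the door's starting relative location.
; Each tick it polls the lever's Active flag to play or reverse a timeline, which lerps the door between that start and OpenZ.
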(event `self.ReceiveBeginPlay`
  (bind _outactors (`GameplayStatics.GetAllActorsOfClass` "/Game/Blueprints/Switches/BP_Lever.BP_Lever_C"))
  (for _array_element _outactors
    (if (== (`/Game/Blueprints/Switches/BP_Lever.LeverIdentifier` _array_element) (`self.DoorIdentifier`))
      (set `self.LeverRef` _array_element)))
  (set `self.DoorInitLocation` (`SceneComponent.RelativeLocation` (`self.Door`)))
  (`self.SetActorTickEnabled` true))

(event `self.ReceiveTick`
  (params (DeltaSeconds :type "Float (single-precision)"))
  (bind _doorinitlocation (`self.DoorInitLocation`))
  (bind _output_get (set `self.bActive` (`/Game/Blueprints/Switches/BP_Lever.bActive` (`self.LeverRef`))))
  (if _output_get
    (bind (_direction _doormovement) (`Timeline|DoorTimeline` :!label _label)
      (:`Update`
        (`SceneComponent.K2_SetRelativeLocation` (`self.Door`) (`KismetMathLibrary.VLerp` _doorinitlocation (`KismetMathLibrary.MakeVector` (.x _doorinitlocation) (.y _doorinitlocation) (`self.OpenZ`)) _doormovement) false false)))
    (else
      (goto _label :!via `Reverse`))))

(fn `UserConstructionScript`)