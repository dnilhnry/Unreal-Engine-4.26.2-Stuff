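; BP_LongPendulumTrapXZ is a pendulum trap that damages the player on contact.
; On BeginPlay it caches player references and applies a one-time acceleration-based force to the WreckingCollumn component, with the Forward flag choosing the sign of InitialForce.
; When the player pawn overlaps KillZone, it prints a red "Player Killed" message and calls ApplyDamage on the ThirdPersonCharacter.
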(event `self.ReceiveBeginPlay`
  (bind _ascharacter (cast `Character` (`GameplayStatics.GetPlayerPawn` 0)))
  (set `self.PlayerRef` _ascharacter)
  (bind _asthird_person_character (cast `/Game/ThirdPersonBP/Blueprints/ThirdPersonCharacter` (`GameplayStatics.GetPlayerCharacter` 0)))
  (set `self.CharacterRef` _asthird_person_character)
  (if (`self.bForward`)
    (set `self.InitialForce` (`self.InitialForce`))
    (else
      (set `self.InitialForce` (* (`self.InitialForce`) -1))))
  (`PrimitiveComponent.AddForce` (`self.WreckingCollumn`) (`self.InitialForce`) "None" true))

(event `self.KillZone.OnComponentBeginOverlap`
  (params (OverlappedComponent :type "PrimitiveComponent Object Reference") (OtherActor :type "Actor Object Reference") (OtherComp :type "PrimitiveComponent Object Reference") (OtherBodyIndex :type Integer) (bFromSweep :type Boolean) (SweepResult :type "HitResult Structure (by ref)"))
  (if (== OtherActor (`self.PlayerRef`))
    (`KismetSystemLibrary.PrintString` "Player Killed" true true (struct :`R` 1.0 :`A` 1.0) 10.0)
    (`/Game/ThirdPersonBP/Blueprints/ThirdPersonCharacter.applyDamage` (`self.CharacterRef`))))

(fn `UserConstructionScript`)