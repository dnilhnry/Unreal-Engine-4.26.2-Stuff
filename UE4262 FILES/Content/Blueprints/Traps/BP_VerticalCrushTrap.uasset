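; Vertical crush trap that moves its ceiling to damage the player after they enter a trigger volume.
; BeginPlay caches the player and ceiling's start position, sets the timeline play rate and resolves an optional delay.
; Trigger overlap waits that delay, then plays a timeline that lerps the ceiling to a fixed relative height.
; Each update, a player overlapping the kill zone receives damage through the third-person character.
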(event `self.ReceiveBeginPlay`
  (bind _ascharacter (cast `Character` (`GameplayStatics.GetPlayerPawn` 0)))
  (set `self.PlayerRef` _ascharacter)
  (bind _asthird_person_character (cast `/Game/ThirdPersonBP/Blueprints/ThirdPersonCharacter` (`GameplayStatics.GetPlayerCharacter` 0)))
  (set `self.CharacterRef` _asthird_person_character)
  (set `self.InitLocation` (`SceneComponent.RelativeLocation` (`self.Ceiling`)))
  (`TimelineComponent.SetPlayRate` (`self.TrapTimeLine`) (`self.PlaySpeed`))
  (if (`self.bHasDealy`)
    (set `self.Delay` (`self.Delay`))
    (else
      (set `self.Delay` 0.0))))

(event `self.Trigger.OnComponentBeginOverlap`
  (params (OverlappedComponent :type "PrimitiveComponent Object Reference") (OtherActor :type "Actor Object Reference") (OtherComp :type "PrimitiveComponent Object Reference") (OtherBodyIndex :type Integer) (bFromSweep :type Boolean) (SweepResult :type "HitResult Structure (by ref)"))
  (bind _initlocation (`self.InitLocation`))
  (`KismetSystemLibrary.Delay` (`self.Delay`))
  (if (== OtherActor (`self.PlayerRef`))
    (bind (_direction _trapmovement) (`Timeline|TrapTimeLine`)
      (:`Update`
        (`SceneComponent.K2_SetRelativeLocation` (`self.Ceiling`) (`KismetMathLibrary.VLerp` _initlocation (`KismetMathLibrary.MakeVector` (.x _initlocation) (.y _initlocation) 150.0) _trapmovement) false false)
        (if (`PrimitiveComponent.IsOverlappingActor` (`self.KillZone`) (`self.PlayerRef`))
          (`KismetSystemLibrary.PrintString` "Player Killed" true true (struct :`R` 1.0 :`A` 1.0) 10.0)
          (`/Game/ThirdPersonBP/Blueprints/ThirdPersonCharacter.applyDamage` (`self.characterRef`)))))))

(fn `UserConstructionScript`)