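; BP_FloorCrumbleTrap is a floor trap that breaks apart when the player character enters its trigger.
; BeginPlay caches the player character and zeroes the delay unless HasDelay is set.
; On overlap by that character, it enables physics on the destructible and activates a radial force.
; After the optional delay it enables gravity on the destructible, separating the break from the fall.
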(event `self.ReceiveBeginPlay`
  (bind _ascharacter (cast `Character` (`GameplayStatics.GetPlayerPawn` 0)))
  (set `self.PlayerRef` _ascharacter)
  (if (`self.bHasDelay`)
    (set `self.Delay` (`self.Delay`))
    (else
      (set `self.Delay` 0.0))))

(event `self.Trigger.OnComponentBeginOverlap`
  (params (OverlappedComponent :type "PrimitiveComponent Object Reference") (OtherActor :type "Actor Object Reference") (OtherComp :type "PrimitiveComponent Object Reference") (OtherBodyIndex :type Integer) (bFromSweep :type Boolean) (SweepResult :type "HitResult Structure (by ref)"))
  (if (== OtherActor (`self.PlayerRef`))
    (`PrimitiveComponent.SetSimulatePhysics` (`self.Destructible`) true)
    (`ActorComponent.Activate` (`self.RadialForce`) false)
    (`KismetSystemLibrary.Delay` (`self.Delay`))
    (`PrimitiveComponent.SetEnableGravity` (`self.Destructible`) true)))

(fn `UserConstructionScript`)