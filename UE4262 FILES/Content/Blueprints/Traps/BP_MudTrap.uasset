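; BP_MudTrap is a trap that slows the player and disables jumping while they stand inside its trigger.
; On BeginPlay it caches the player character, its movement component, and the original walk speed and jump velocity.
; Trigger overlap lowers walk speed and zeroes jump velocity for that player only, and end overlap restores the cached values.
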(event `self.ReceiveBeginPlay`
  (bind _ascharacter (cast `Character` (`GameplayStatics.GetPlayerPawn` 0)))
  (bind _output_get (set `self.PlayerRef` _ascharacter))
  (bind _output_get_2 (set `self.PlayerMovement` (`Character.CharacterMovement` _output_get)))
  (set `self.InitWalkSpeed` (`CharacterMovementComponent.MaxWalkSpeed` _output_get_2))
  (set `self.InitJumpVelocity` (`CharacterMovementComponent.JumpZVelocity` _output_get_2)))

(event `self.Trigger.OnComponentBeginOverlap`
  (params (OverlappedComponent :type "PrimitiveComponent Object Reference") (OtherActor :type "Actor Object Reference") (OtherComp :type "PrimitiveComponent Object Reference") (OtherBodyIndex :type Integer) (bFromSweep :type Boolean) (SweepResult :type "HitResult Structure (by ref)"))
  (bind _playermovement (`self.PlayerMovement`))
  (if (== OtherActor (`self.PlayerRef`))
    (set `CharacterMovementComponent.MaxWalkSpeed` 100.0 _playermovement)
    (set `CharacterMovementComponent.JumpZVelocity` 0.0 _playermovement)))

(event `self.Trigger.OnComponentEndOverlap`
  (params (OverlappedComponent :type "PrimitiveComponent Object Reference") (OtherActor :type "Actor Object Reference") (OtherComp :type "PrimitiveComponent Object Reference") (OtherBodyIndex :type Integer))
  (bind _playermovement (`self.PlayerMovement`))
  (if (== OtherActor (`self.PlayerRef`))
    (set `CharacterMovementComponent.MaxWalkSpeed` (`self.InitWalkSpeed`) _playermovement)
    (set `CharacterMovementComponent.JumpZVelocity` (`self.InitJumpVelocity`) _playermovement)))

(fn `UserConstructionScript`)