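; A bridge actor that raises or lowers along Z according to the state of a linked lever.
; On BeginPlay it searches all BP_Lever actors and stores the one whose LeverIdentifier matches its own BridgeIdentifier.
; Every Tick it polls that lever's Active flag to play or reverse a timeline, which lerps the bridge's relative location between its initial position and OpenZ.
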(event `self.ReceiveBeginPlay`
  (bind _outactors (`GameplayStatics.GetAllActorsOfClass` "/Game/Blueprints/Switches/BP_Lever.BP_Lever_C"))
  (for _array_element _outactors
    (if (== (`/Game/Blueprints/Switches/BP_Lever.LeverIdentifier` _array_element) (`self.BridgeIdentifier`))
      (set `self.LeverRef` _array_element)))
  (`self.SetActorTickEnabled` true))

(event `self.ReceiveTick`
  (params (DeltaSeconds :type "Float (single-precision)"))
  (bind _bridgeinitlocation (`self.BridgeInitLocation`))
  (bind _output_get (set `self.bActive` (`/Game/Blueprints/Switches/BP_Lever.bActive` (`self.LeverRef`))))
  (if _output_get
    (bind (_direction _bridgemovement) (`Timeline|BridgeTimeline` :!label _label)
      (:`Update`
        (`SceneComponent.K2_SetRelativeLocation` (`self.Bridge`) (`KismetMathLibrary.VLerp` _bridgeinitlocation (`KismetMathLibrary.MakeVector` (.x _bridgeinitlocation) (.y _bridgeinitlocation) (`self.OpenZ`)) _bridgemovement) false false)))
    (else
      (goto _label :!via `Reverse`))))

(fn `UserConstructionScript`)