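; Moving platform actor that slides two platforms back and forth along their relative X axis.
; On BeginPlay it stores both starting locations, then a timeline lerps Platform0 to plus half of TravelDistance and Platform1 to minus half, keeping Y and Z.
; When the timeline finishes, it compares Platform0's rounded X, doubled, to TravelDistance to choose between reversing and replaying, creating an endless ping-pong.
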(event `self.ReceiveBeginPlay`
  (bind (_initlocation1_x _initlocation1_y _initlocation1_z) (`KismetMathLibrary.BreakVector` (`self.InitLocation1`)))
  (bind (_initlocation0_x _initlocation0_y _initlocation0_z) (`KismetMathLibrary.BreakVector` (`self.InitLocation0`)))
  (bind _relativelocation_x (`KismetMathLibrary.BreakVector` (`SceneComponent.RelativeLocation` (`self.Platform0`))))
  (set `self.InitLocation0` (`SceneComponent.RelativeLocation` (`self.Platform0`)))
  (set `self.InitLocation1` (`SceneComponent.RelativeLocation` (`self.Platform1`)))
  (bind (_direction _platfrommovement) (`Timeline|PlatfromTimeline` :!via `PlayFromStart` :!label _label)
    (:`Update`
      (`SceneComponent.K2_SetRelativeLocation` (`self.Platform0`) (`KismetMathLibrary.VLerp` (`KismetMathLibrary.MakeVector` _initlocation0_x _initlocation0_y _initlocation0_z) (`KismetMathLibrary.MakeVector` (/ (`self.TravelDistance`) 2.0) (.y (`KismetMathLibrary.MakeVector` 0.0 _initlocation0_y _initlocation0_z)) (.z (`KismetMathLibrary.MakeVector` 0.0 _initlocation0_y _initlocation0_z))) _platfrommovement) false false)
      (`SceneComponent.K2_SetRelativeLocation` (`self.Platform1`) (`KismetMathLibrary.VLerp` (`KismetMathLibrary.MakeVector` _initlocation1_x _initlocation1_y _initlocation1_z) (`KismetMathLibrary.MakeVector` (/ (`self.TravelDistance`) -2.0) (.y (`KismetMathLibrary.MakeVector` 0.0 _initlocation1_y _initlocation1_z)) (.z (`KismetMathLibrary.MakeVector` 0.0 _initlocation1_y _initlocation1_z))) _platfrommovement) false false))
    (:`Finished`
      (if (== (* (`KismetMathLibrary.Conv_IntToDouble` (`KismetMathLibrary.Round` _relativelocation_x)) 2.0) (`self.TravelDistance`))
        (goto _label :!via `ReverseFromEnd`)
        (else
          (goto _label :!via `PlayFromStart`))))))

(fn `UserConstructionScript`)