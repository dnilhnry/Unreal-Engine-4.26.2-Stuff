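; A lever switch actor that the player toggles with the Interact input while inside its trigger volume.
; Trigger overlap prints a prompt and opens a gate for the input, and leaving closes it.
; Interact plays an on or off timeline that lerps the lever's rotation and flips Active when finished.
; Tick re-enters BeginPlay's logic, reapplying the rotation for the current Active state and re-enabling input every frame, even during timelines.
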(event `self.ReceiveBeginPlay`
  (bind _ascharacter (cast `Character` (`GameplayStatics.GetPlayerPawn` 0)))
  (set `self.PlayerRef` _ascharacter)
  (`self.SetActorTickEnabled` true)
  (if (`self.bActive`) :!label _label
    (`SceneComponent.K2_SetRelativeRotation` (`self.Lever`) (`self.OnRotator`) false false)
    (else
      (`SceneComponent.K2_SetRelativeRotation` (`self.Lever`) (`self.OffRotator`) false false)))
  (`self.EnableInput` (`GameplayStatics.GetPlayerController` 0)))

(event `self.ReceiveTick`
  (params (DeltaSeconds :type "Float (single-precision)"))
  (goto _label))

(event `InputAction|Interact` :consume false
  (params (Key :type "Key Structure"))
  (:`Pressed`
    (`/Engine/EditorBlueprintResources/StandardMacros.Gate` true :!label _label_2
      (:`Exit`
        (if (`self.bActive`)
          (bind (_direction _levermovement) (`Timeline|LeverTimelineOff` :!via `PlayFromStart`)
            (:`Update`
              (`SceneComponent.K2_SetRelativeRotation` (`self.Lever`) (`KismetMathLibrary.RLerp` (`self.OnRotator`) (`self.OffRotator`) _levermovement) false false))
            (:`Finished`
              (set `self.bActive` false)))
          (else
            (bind (_direction_2 _levermovement_2) (`Timeline|LeverTimelineOn` :!via `PlayFromStart`)
              (:`Update`
                (`SceneComponent.K2_SetRelativeRotation` (`self.Lever`) (`KismetMathLibrary.RLerp` (`self.OffRotator`) (`self.OnRotator`) _levermovement_2) false false))
              (:`Finished`
                (set `self.bActive` true)))))))))

(event `self.Trigger.OnComponentBeginOverlap`
  (params (OverlappedComponent :type "PrimitiveComponent Object Reference") (OtherActor :type "Actor Object Reference") (OtherComp :type "PrimitiveComponent Object Reference") (OtherBodyIndex :type Integer) (bFromSweep :type Boolean) (SweepResult :type "HitResult Structure (by ref)"))
  (if (== OtherActor (`self.PlayerRef`))
    (`KismetSystemLibrary.PrintString` "Press 'E' To Interact" true true (struct :`G` 0.66 :`B` 1.0 :`A` 1.0) 5.0)
    (goto _label_2 :!via `Open`)))

(event `self.Trigger.OnComponentEndOverlap`
  (params (OverlappedComponent :type "PrimitiveComponent Object Reference") (OtherActor :type "Actor Object Reference") (OtherComp :type "PrimitiveComponent Object Reference") (OtherBodyIndex :type Integer))
  (if (== OtherActor (`self.PlayerRef`))
    (goto _label_2 :!via `Close`)))

(fn `UserConstructionScript`)